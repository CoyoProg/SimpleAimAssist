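; BP_HealthComponent is a health component that receives damage and reports whether its owner is alive.
; TakeDamage doubles the incoming amount when the BodyPart variable is Head or Apple, then passes the final amount out through CallOnHit.
; The shown graphs only read IsDead for the alive check and neither subtract health nor set the death state.
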(fn `IsAlive`
  (returns (`bIsAlive?` :type Boolean))
  (return (not (`self.bIsDead`))))

(fn `TakeDamage`
  (params (DamageAmount :type Integer))
  (locals (FinalDamageAmount :type Integer))
  (set `local.FinalDamageAmount` DamageAmount)
  (`|ExecutionSequence`
    (:`then_0`
      (switch `/Game/SimpleAimAssist/Demo/Blueprints/ShootingTarget/E_BodyParts` (`self.BodyPart`)
        (:`NewEnumerator1`
          _)
        (:`NewEnumerator2`
          _))
      (set `local.FinalDamageAmount` (* DamageAmount 2)))
    (:`then_1`
      (`self.OnHit` (`local.FinalDamageAmount`)))))