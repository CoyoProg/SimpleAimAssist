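; HUD-owned debug component that visualizes aim assist radius circles and crosshair state while debug is enabled.
; InitializeCircles builds one colored dynamic material per circle, while events update radii, crosshair location, color, state text and screen size.
; ReceiveDrawHUD draws screen-centered circles, then the state text and crosshair, offset vertically for the HUD-to-game viewport difference.
; The crosshair material instance is recreated on every draw.
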(event `self.ReceiveBeginPlay`
  (`self.GetOwnerHUD`))

(event `ToggleVisualizer`
  (params (bShouldEnable :type Boolean))
  (set `self.IsDebugEnabled` bShouldEnable))

(event `OnCrossHairUpdate`
  (params (AdjustedCrossHairLocation :type "Vector2D Structure") (CurrentColor :type "LinearColor Structure") (AssistState :type String))
  (`|ExecutionSequence`
    (:`then_0`
      (set `self.CrossHairLocation` AdjustedCrossHairLocation))
    (:`then_1`
      (set `self.ColorCurrentState` CurrentColor))
    (:`then_2`
      (set `self.AssistState` AssistState))))

(event `UpdateScreenSizeValue`
  (params (ViewportSize :type "Vector2D Structure"))
  (set `self.ScreenSize` ViewportSize))

(event `ReceiveDrawHUD`
  (params (SizeX :type Integer) (SizeY :type Integer))
  ;[1 1 1 0.33] Get HUD Screen Size
  (if (`self.IsDebugEnabled`)
    (bind _output_get (set `self.HUDViewportSize` (`KismetMathLibrary.MakeVector2D` (`KismetMathLibrary.Conv_IntToDouble` SizeX) (`KismetMathLibrary.Conv_IntToDouble` SizeY))))
    (bind (_returnvalue_x _returnvalue_y) (`KismetMathLibrary.BreakVector2D` (- (`self.ScreenSize`) _output_get)))
    ;[1 1 1 0.33] Get Y Offset, difference from HUD Viewport & GameViewport
    (set `self.OffsetVIewportY` (/ _returnvalue_y 2.0))
    ;[1 1 1 0.33] Draw Each Circles
    (for (_array_element _array_index) (`self.CirclesMI`)
      (`self.DrawCircle` _array_element (`|GetArrayItem` (`self.Radiuses`) _array_index)))
    ;[1 1 1 0.33] Draw and Update CrossHair Location
    (`self.DrawCross` (- (`self.CrossHairLocation`) (`KismetMathLibrary.MakeVector2D` 0.0 (`self.OffsetVIewportY`))) (`self.AssistState`) (`self.ColorCurrentState`) 10.0)))

(event `OnCircleUpdate`
  (params (InRadius :type "Array of Float (double-precision)"))
  (for (_array_element _array_index) InRadius
    (`KismetArrayLibrary.Array_Set` (`self.Radiuses`) _array_index _array_element)))

(fn `DrawCircle`
  (params (Material :type "MaterialInterface Object Reference") (Radius :type "Float (double-precision)"))
  (bind _returnvalue (* Radius 2.0))
  (bind (_returnvalue_x _returnvalue_y) (`KismetMathLibrary.BreakVector2D` (- (/ (`self.HUDViewportSize`) (2.0 2.0)) (`KismetMathLibrary.MakeVector2D` Radius Radius))))
  (`HUD.DrawMaterialSimple` (`self.OwnerHUD`) Material _returnvalue_x _returnvalue_y _returnvalue _returnvalue 1.0 false))

(fn `DrawCross`
  (params (ScreenLocation :type "Vector2D Structure") (InText :type String) (InColor :type "LinearColor Structure") (InSize :type "Float (double-precision)"))
  (bind (_returnvalue_x _returnvalue_y) (`KismetMathLibrary.BreakVector2D` (- ScreenLocation (0.0 0.0))))
  (bind _insize (`local.InSize`))
  (bind _returnvalue (/ (`local.InSize`) 2.0))
  (bind (_returnvalue_x_2 _returnvalue_y_2) (`KismetMathLibrary.BreakVector2D` (- (`local.ScreenLocation`) (`KismetMathLibrary.MakeVector2D` _returnvalue _returnvalue))))
  (`HUD.DrawText` (`self.OwnerHUD`) (`local.InText`) (`local.InColor`) _returnvalue_x _returnvalue_y null 1.5 false)
  (bind _returnvalue_2 (`KismetMaterialLibrary.CreateDynamicMaterialInstance` "/Game/SimpleAimAssist/Debug/M_DebugCrossHair.M_DebugCrossHair"))
  (set `self.CrossHairMI` _returnvalue_2)
  (`|ExecutionSequence`
    (:`then_0`
      (`MaterialInstanceDynamic.SetVectorParameterValue` (`self.CrossHairMI`) "Color" (`local.InColor`)))
    (:`then_1`
      (`MaterialInstanceDynamic.SetScalarParameterValue` (`self.CrossHairMI`) "TextureSize" (`local.InSize`)))
    (:`then_2`
      (`MaterialInstanceDynamic.SetScalarParameterValue` (`self.CrossHairMI`) "LineSmoothingSize" (`self.CrossHairSmoothing`)))
    (:`then_3`
      (`MaterialInstanceDynamic.SetScalarParameterValue` (`self.CrossHairMI`) "LineWidth" (`self.CrossHairLineWidth`))
      (`HUD.DrawMaterialSimple` (`self.OwnerHUD`) (`self.CrossHairMI`) _returnvalue_x_2 _returnvalue_y_2 _insize _insize 1.0 false))))

(fn `GetOwnerHUD`
  (bind _ashud (cast `HUD` (`self.GetOwner`)))
  (set `self.OwnerHUD` _ashud))

(fn `InitializeCircles`
  (params (InRadiuses :type "Array of Float (double-precision)"))
  (locals (MaterialInstance :type "MaterialInstanceDynamic Object Reference") (Colors :type "Array of LinearColor Structure") (CurrentColor :type "LinearColor Structure"))
  (set `self.Radiuses` InRadiuses)
  (`KismetArrayLibrary.Array_Clear` (`self.CirclesMI`))
  (for (_array_element _array_index) (`local.Colors`)
    (bind _returnvalue (`KismetMaterialLibrary.CreateDynamicMaterialInstance` "/Game/SimpleAimAssist/Debug/M_DebugCircle.M_DebugCircle"))
    (set `local.MaterialInstance` _returnvalue)
    (`|ExecutionSequence`
      (:`then_0`
        (`MaterialInstanceDynamic.SetVectorParameterValue` (`local.MaterialInstance`) "Color" _array_element))
      (:`then_1`
        (`MaterialInstanceDynamic.SetScalarParameterValue` (`local.MaterialInstance`) "TextureSize" (* (`|GetArrayItem` (`self.Radiuses`) _array_index) 2.0)))
      (:`then_2`
        (`MaterialInstanceDynamic.SetScalarParameterValue` (`local.MaterialInstance`) "LineThickness" (`self.CircleThickness`)))
      (:`then_3`
        (`MaterialInstanceDynamic.SetScalarParameterValue` (`local.MaterialInstance`) "LineSmoothingSize" (`self.CircleSmoothing`))
        (`KismetArrayLibrary.Array_AddUnique` (`self.CirclesMI`) (`local.MaterialInstance`))))))