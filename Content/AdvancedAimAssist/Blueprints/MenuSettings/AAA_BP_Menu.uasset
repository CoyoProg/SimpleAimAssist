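; AAA_BP_Menu is an in-world settings menu for the Advanced Aim Assist system, built from AAA_MenuButton child actors.
; One tick after BeginPlay it finds the player pawn's aim assist component and hands it to the master button and the buttons nested under it.
; The master button's disable event resets, disables and locks the nested buttons, while its enable event only unlocks them.
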(event `self.ReceiveBeginPlay`
  (bind _returnvalue (`self.GetComponentByClass` (`GameplayStatics.GetPlayerPawn` 0) "/Game/AdvancedAimAssist/Blueprints/Components/AAA_BP_AimAssistComponent.AAA_BP_AimAssistComponent_C"))
  ;[1 0 0.02407 0.25] BEGIN PLAY
  (`KismetSystemLibrary.DelayUntilNextTick`)
  (`/Engine/EditorBlueprintResources/StandardMacros.IsValid` _returnvalue
    (:`Is Valid`
      (set `self.AimAssistComponent` _returnvalue)
      (for _array_element (`SceneComponent.GetChildrenComponents` (`self.ChildActor`) false)
        (bind _aschild_actor_component (cast `ChildActorComponent` _array_element))
        (bind _asaaa_menu_button (cast `/Game/AdvancedAimAssist/Blueprints/MenuSettings/AAA_MenuButton` (`ChildActorComponent.ChildActor` _aschild_actor_component)))
        (`KismetArrayLibrary.Array_AddUnique` (`self.Buttons`) _asaaa_menu_button)
        (set `/Game/AdvancedAimAssist/Blueprints/MenuSettings/AAA_MenuButton.AimAssistComp` (`self.AimAssistComponent`) _asaaa_menu_button))
      (bind _asaaa_menu_button_2 (cast `/Game/AdvancedAimAssist/Blueprints/MenuSettings/AAA_MenuButton` (`ChildActorComponent.ChildActor` (`self.ChildActor`))))
      (add `/Game/AdvancedAimAssist/Blueprints/MenuSettings/AAA_MenuButton.OnAimAssistDisable` _asaaa_menu_button_2 (delegate `DisableAll`))
      (add `/Game/AdvancedAimAssist/Blueprints/MenuSettings/AAA_MenuButton.OnAimAssistEnable` _asaaa_menu_button_2 (delegate `UnlockAll`))
      (set `/Game/AdvancedAimAssist/Blueprints/MenuSettings/AAA_MenuButton.AimAssistComp` (`self.AimAssistComponent`) _asaaa_menu_button_2))))

(event `DisableAll`
  ;[1 0 0.02407 0.25] DISABLE Butons
  (for _array_element (`self.Buttons`)
    (set `/Game/AdvancedAimAssist/Blueprints/MenuSettings/AAA_MenuButton.CurrentIndex` 0 _array_element)
    (`/Game/AdvancedAimAssist/Blueprints/MenuSettings/AAA_MenuButton.DisableButton` _array_element)
    (set `/Game/AdvancedAimAssist/Blueprints/MenuSettings/AAA_MenuButton.bIsLocked` true _array_element)))

(event `UnlockAll`
  ;[1 0 0.02407 0.25] UNLOCK Buttons
  (for _array_element (`self.Buttons`)
    (set `/Game/AdvancedAimAssist/Blueprints/MenuSettings/AAA_MenuButton.bIsLocked` false _array_element)))

(fn `UserConstructionScript`)