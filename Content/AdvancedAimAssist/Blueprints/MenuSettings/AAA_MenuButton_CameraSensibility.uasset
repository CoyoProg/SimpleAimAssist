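; AAA_MenuButton_CameraSensibility is a hit-activated menu button that adjusts the first-person player's camera sensitivity.
; On BeginPlay it caches the AAA_BP_FirstPersonPlayer pawn, or resets its index and disables itself if the cast fails.
; Each hit on HitComponent advances a wrapping index, which is scaled and clamped into the same sensitivity for both axes before the button text updates.
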(event `self.ReceiveBeginPlay`
  (bind _asaaa_bp_first_person_player (cast `/Game/AdvancedAimAssist/UnrealFPS/Blueprints/AAA_BP_FirstPersonPlayer` (`GameplayStatics.GetPlayerPawn` 0))
    (:`then`
      (set `self.PlayerFPS` _asaaa_bp_first_person_player))
    (:`CastFailed`
      (set `self.CurrentIndex` 0)
      (`self.DisableButton`))))

(event `self.HitComponent.OnHit`
  (params (DamageAmount :type Integer))
  (bind _returnvalue (`KismetMathLibrary.FClamp` (/ (`self.CurrentIndex`) 10) 0.1))
  (bind _result (`/Engine/EditorBlueprintResources/StandardMacros.IncrementInt` (`self.CurrentIndex`))
    (:`  `
      (if (> _result 10)
        (set `self.CurrentIndex` 1))
      (bind _playerfps (`self.PlayerFPS`)
        (:`then`
          (set `/Game/AdvancedAimAssist/UnrealFPS/Blueprints/AAA_BP_FirstPersonPlayer.CameraSensitivity` (`KismetMathLibrary.MakeVector2D` _returnvalue _returnvalue) _playerfps)
          (`self.UpdateText`))
        (:`else`)))))

(fn `UserConstructionScript`
  (`parent.UserConstructionScript`))