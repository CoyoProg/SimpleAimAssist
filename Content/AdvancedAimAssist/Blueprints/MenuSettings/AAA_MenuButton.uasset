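; AAA_MenuButton is a text-render menu button in the Advanced Aim Assist settings menu that displays one option from a list of setting labels.
; EnableButton and DisableButton switch the TextRender component between the enabled and disabled colors, then refresh its text.
; UpdateText shows the TextSettings entry at CurrentIndex; no graph here changes that index or handles input.
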(fn `DisableButton`
  (`TextRenderComponent.SetTextRenderColor` (`self.TextRender`) (`self.DisableColor`))
  (`self.UpdateText`))

(fn `EnableButton`
  (`TextRenderComponent.SetTextRenderColor` (`self.TextRender`) (`self.EnableColor`))
  (`self.UpdateText`))

(fn `UpdateText`
  (`TextRenderComponent.K2_SetText` (`self.TextRender`) (`|GetArrayItem` (`self.TextSettings`) (`self.CurrentIndex`))))

(fn `UserConstructionScript`)