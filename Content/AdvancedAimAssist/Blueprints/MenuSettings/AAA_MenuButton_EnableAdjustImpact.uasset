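; Shootable menu button for the Advanced Aim Assist settings that toggles bullet magnetism (impact adjustment) on the aim assist component.
; When unlocked, each hit on its HitComponent advances a two-state index that wraps around and calls DisableButton or EnableButton if the component is valid.
; Both overrides run the parent logic, then set EnableBulletMagnetism; the enable path also refreshes the button text.
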(event `self.HitComponent.OnHit`
  (params (DamageAmount :type Integer))
  (if (not (`self.bIsLocked`))
    (bind _result (`/Engine/EditorBlueprintResources/StandardMacros.IncrementInt` (`self.CurrentIndex`))
      (:`  `
        (if (> _result 1)
          (set `self.CurrentIndex` 0))
        (`self.AimAssistComp`
          (:`then`
            (switch `int` (`self.CurrentIndex`)
              (:`0`
                (`self.DisableButton`))
              (:`1`
                (`self.EnableButton`))))
          (:`else`))))))

(fn `DisableButton`
  (`parent.DisableButton`)
  (set `/Game/AdvancedAimAssist/Blueprints/Components/AAA_BP_AimAssistComponent.bEnableBulletMagnetism` false (`self.AimAssistComp`)))

(fn `EnableButton`
  (`parent.EnableButton`)
  (set `/Game/AdvancedAimAssist/Blueprints/Components/AAA_BP_AimAssistComponent.bEnableBulletMagnetism` true (`self.AimAssistComp`))
  (`self.UpdateText`))

(fn `UserConstructionScript`
  (`parent.UserConstructionScript`))