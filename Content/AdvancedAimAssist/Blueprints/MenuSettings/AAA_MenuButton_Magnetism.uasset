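; Menu button in the Advanced Aim Assist settings that cycles camera magnetism between off and two strengths.
; When hit and not locked, it advances a wrapping index and writes the matching CameraMagneticForce to the aim assist component.
; The off state runs through a DisableButton override that zeroes the force, while the active states enable the button or refresh its text.
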(event `self.HitComponent.OnHit`
  (params (DamageAmount :type Integer))
  (if (not (`self.bIsLocked`))
    (bind _result (`/Engine/EditorBlueprintResources/StandardMacros.IncrementInt` (`self.CurrentIndex`))
      (:`  `
        (if (> _result 2)
          (set `self.CurrentIndex` 0))
        (`self.AimAssistComp`
          (:`then`
            (switch `int` (`self.CurrentIndex`)
              (:`0`
                (`self.DisableButton`))
              (:`1`
                (`self.EnableButton`)
                (set `/Game/AdvancedAimAssist/Blueprints/Components/AAA_BP_AimAssistComponent.CameraMagneticForce` 0.1 (`self.AimAssistComp`)))
              (:`2`
                (set `/Game/AdvancedAimAssist/Blueprints/Components/AAA_BP_AimAssistComponent.CameraMagneticForce` 0.2 (`self.AimAssistComp`))
                (`self.UpdateText`))))
          (:`else`))))))

(fn `DisableButton`
  (`parent.DisableButton`)
  (set `/Game/AdvancedAimAssist/Blueprints/Components/AAA_BP_AimAssistComponent.CameraMagneticForce` 0.0 (`self.AimAssistComp`)))

(fn `UserConstructionScript`
  (`parent.UserConstructionScript`))