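; Menu button that toggles the Advanced Aim Assist component, built on a parent button class and triggered by hits on its hit component.
; Each hit cycles an index through three states: disabled, enabled, and enabled with debug.
; Disabling stops aim assist and clears debug, and the off and on states fire the disable and enable dispatchers.
; With a valid component, every hit ends by initializing the HUD.
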(event `self.HitComponent.OnHit`
  (params (DamageAmount :type Integer))
  (bind _result (`/Engine/EditorBlueprintResources/StandardMacros.IncrementInt` (`self.CurrentIndex`))
    (:`  `
      (if (> _result 2)
        (set `self.CurrentIndex` 0))
      (bind _aimassistcomp (`self.AimAssistComp`)
        (:`then`
          (`|ExecutionSequence`
            (:`then_0`
              (switch `int` (`self.CurrentIndex`)
                (:`0`
                  (`self.DisableButton`)
                  (`self.OnAimAssistDisable`))
                (:`1`
                  (`/Game/AdvancedAimAssist/Blueprints/Components/AAA_BP_AimAssistComponent.StartAimAssist` (`self.AimAssistComp`))
                  (`self.OnAimAssistEnable`)
                  (`self.EnableButton` :!label _label))
                (:`2`
                  (set `/Game/AdvancedAimAssist/Blueprints/Components/AAA_BP_AimAssistComponent.bIsDebugActivated` true (`self.AimAssistComp`))
                  (goto _label))))
            (:`then_1`
              (`/Game/AdvancedAimAssist/Blueprints/Components/AAA_BP_AimAssistComponent.Initialize HUD` _aimassistcomp))))
        (:`else`)))))

(fn `DisableButton`
  (bind _aimassistcomp (`self.AimAssistComp`))
  (`parent.DisableButton`)
  (set `/Game/AdvancedAimAssist/Blueprints/Components/AAA_BP_AimAssistComponent.bIsDebugActivated` false _aimassistcomp)
  (`/Game/AdvancedAimAssist/Blueprints/Components/AAA_BP_AimAssistComponent.StopAimAssist` _aimassistcomp))

(fn `UserConstructionScript`
  (`parent.UserConstructionScript`))