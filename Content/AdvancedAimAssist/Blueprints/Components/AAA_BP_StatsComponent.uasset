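; Stats component for an aim-assist game that tracks shots, hits, misses, accuracy and score, with a floating points popup.
; UpdateScore awards points by body part (body, head or apple) and fires OnScoreUpdated.
; A text render created at BeginPlay is placed near each impact, nudged toward and facing the owner, and scaled by distance.
; PopupFX moves it vertically and sets opacity through a dynamic material, using values from the caller.
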(event `self.ReceiveBeginPlay`
  (bind _returnvalue (`|AddComponentByClass` :`self` (`self.GetOwner`) :`Class` "/Script/Engine.TextRenderComponent" :`bManualAttachment` true))
  (bind _output_get (set `self.ScorePopUp` _returnvalue))
  (`TextRenderComponent.K2_SetText` _output_get (`|FormatText` ""))
  (`TextRenderComponent.SetTextMaterial` _output_get "/Game/AdvancedAimAssist/ART/Materials/DefaultTextMaterialEmissive.DefaultTextMaterialEmissive")
  (`TextRenderComponent.SetTextRenderColor` _output_get (`self.PopupColor`))
  (bind _returnvalue_2 (`PrimitiveComponent.CreateDynamicMaterialInstance` (`self.ScorePopUp`) 0 (`PrimitiveComponent.GetMaterial` _output_get 0) "None"))
  (set `self.MatInst` _returnvalue_2))

(event `OnMiss`
  (`/Engine/EditorBlueprintResources/StandardMacros.IncrementFloat` (`self.TotalMisses`)
    (:`  `
      (`/Engine/EditorBlueprintResources/StandardMacros.IncrementFloat` (`self.TotalShots`) :!label _label
        (:`  `
          (set `self.AccuracyStats` (* (/ (`self.TotalHits`) (`self.TotalShots`)) 100.0)))))))

(event `OnHit`
  (`/Engine/EditorBlueprintResources/StandardMacros.IncrementFloat` (`self.TotalHits`)
    (:`  `
      (goto _label))))

(event `UpdateScore`
  (params (BodyPart :type "/Game/AdvancedAimAssist/Blueprints/ShootingTarget/AAA_E_BodyParts Enum" :default "NewEnumerator3"))
  (switch `/Game/AdvancedAimAssist/Blueprints/ShootingTarget/AAA_E_BodyParts` BodyPart
    (:`NewEnumerator3`
      (set `self.PointAmount` 0))
    (:`NewEnumerator0`
      (set `self.PointAmount` 100)
      (set `self.Score` (+ (`self.PointAmount`) (`self.Score`)) :!label _label_2)
      (`self.OnScoreUpdated`))
    (:`NewEnumerator1`
      (set `self.PointAmount` 500)
      (goto _label_2))
    (:`NewEnumerator2`
      (set `self.PointAmount` 1000)
      (goto _label_2))))

(event `UpdatePopupLocation`
  (params (ImpactLocation :type "Vector Structure"))
  (bind _pointamount (`self.PointAmount`))
  (bind _scorepopup (`self.ScorePopUp`))
  (bind _returnvalue (- (`Actor.K2_GetActorLocation` (`self.GetOwner`)) ImpactLocation))
  (bind _returnvalue_2 (`KismetMathLibrary.FClamp` (/ (`KismetMathLibrary.VSize` _returnvalue) 1000.0) 1.0 5.0))
  (bind _returnvalue_3 (+ (* (`KismetMathLibrary.Normal` _returnvalue) 10) ImpactLocation))
  (`SceneComponent.SetWorldScale3D` (`self.ScorePopUp`) (`KismetMathLibrary.MakeVector` _returnvalue_2 _returnvalue_2 _returnvalue_2))
  (`SceneComponent.K2_SetWorldLocation` (`self.ScorePopUp`) _returnvalue_3 false false)
  (`SceneComponent.K2_SetWorldRotation` (`self.ScorePopUp`) (`KismetMathLibrary.FindLookAtRotation` _returnvalue_3 (`Actor.K2_GetActorLocation` (`self.GetOwner`))) false false)
  (if (!= _pointamount 0)
    (`TextRenderComponent.K2_SetText` _scorepopup (`KismetTextLibrary.Conv_StringToText` (`KismetStringLibrary.Concat_StrStr` "+ " (`KismetTextLibrary.Conv_TextToString` (`KismetTextLibrary.Conv_IntToText` _pointamount)))))
    (else
      (`TextRenderComponent.K2_SetText` _scorepopup (`|FormatText` "")))))

(event `PopupFX`
  (params (Delta :type "Float (double-precision)") (Alpha :type "Float (double-precision)"))
  (`SceneComponent.K2_AddWorldOffset` (`self.ScorePopUp`) (`KismetMathLibrary.MakeVector` 0.0 0.0 Delta) false false)
  (`MaterialInstanceDynamic.SetScalarParameterValue` (`self.MatInst`) "Opacity" (/ Alpha 10.0)))

(fn `ResetStats`
  (set `self.AccuracyStats` 0.0)
  (set `self.TotalShots` 0.0)
  (set `self.TotalMisses` 0.0)
  (set `self.TotalHits` 0.0)
  (set `self.Score` 0))