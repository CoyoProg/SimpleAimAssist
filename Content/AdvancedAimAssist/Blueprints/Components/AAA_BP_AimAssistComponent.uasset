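; Aim assist component that provides camera stickiness, snap and bullet magnetism toward nearby Pawns.
; While look input triggers it, Tick sphere-traces from screen center and picks a target by screen distance and input alignment.
; Distance-scaled screen radii drive camera deceleration and yaw/pitch pull, while AdjustImpactPoint returns a magnetized shot direction.
; Near-zero input starts a timer that releases the lock; an optional debug HUD displays zones and state.
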(event `self.ReceiveBeginPlay`
  ;[1 0.02791 0 0.25] BEGIN PLAY
  ;;[1 1 1] Get Player Controller Reference & Initialize HUD
  (`self.GetPlayerController`)
  (`self.Initialize HUD`))

(event `self.ReceiveTick`
  (params (DeltaSeconds :type "Float (single-precision)"))
  ;[1 0 0.02461 0.25] Check if AimAssist is Enable
  (if (`self.bIsAimAssistEnable`)
    (`|ExecutionSequence`
      (:`then_0`
        ;[1 0 0.02461 0.25] Check if Aim Assist is Triggered
        (if (`self.bIsAimAssistTriggered`)
          ;[1 1 1 0.33] Find closest hit
          (bind (_hit_ _hitscreenlocation) (`self.Enemy Detection`))
          (`|ExecutionSequence`
            (:`then_0`
              ;[1 0 0.02461 0.25] Check if there is a hit
              (if _hit_
                ;[1 1 1 0.33] Adjust CrossHair
                (bind _adjustedcrosshair (`self.AdjustPlayerAim` _hitscreenlocation))
                (set `self.AdjustCrossHairLocatin` _adjustedcrosshair)
                (else
                  ;[1 1 1 0.33] Reset Camera
                  (`self.ResetCamera`))))
            (:`then_1`
              ;[1 1 1 0.33] Update Debug AimAssist HUD
              (`self.UpdateHUD`)))))
      (:`then_1`
        ;[1 1 1 0.25] Update Lock Target State Timer
        ;;[1 0 0.02461 0.25] Check if low Velocity
        (if (`self.bTriggerLowVelocity`)
          (`self.UpdateLockState` DeltaSeconds)))
      (:`then_2`
        ;[1 1 1 0.25] Update Screen Center and Screen Size of HUD
        (`KismetSystemLibrary.Delay` 0.2)
        (`self.UpdateScreenCenter`)))))

(fn `AdjustCircles`
  (params (CurrentTarget :type "Vector Structure"))
  (locals (DistanceRatio :type "Float (double-precision)"))
  ;[1 1 1 0.25] Get Target distance ratio from  Player
  (set `local.DistanceRatio` (- 1.0 (/ (`KismetMathLibrary.Vector_Distance` CurrentTarget (`Actor.K2_GetActorLocation` (`Controller.K2_GetPawn` (`self.PlayerController`)))) (`self.SphereTraceRange`))))
  ;[1 1 1 0.25] Adjust aim assist Zones depending on the Distance Ratio
  (`|ExecutionSequence`
    (:`then_0`
      (set `self.Adjusted_CS_Radius` (* (`self.CameraSnapRadius`) (`local.DistanceRatio`))))
    (:`then_1`
      (set `self.Adjusted_BM_Radius` (* (`self.BulletMagnetismRadius`) (`local.DistanceRatio`))))
    (:`then_2`
      (set `self.Adjusted_S_Radius` (* (`self.SticknessRadius`) (`local.DistanceRatio`))))
    (:`then_3`
      ;[1 1 1 0.25] Update Circles HUD
      (if (`self.bIsDebugActivated`)
        (`/Game/AdvancedAimAssist/Debug/AAA_HUD_Debug.OnCircleUpdate` (`self.AimAssistHUD`) (`|MakeArray` (`self.Adjusted_BM_Radius`) (`self.Adjusted_CS_Radius`) (`self.Adjusted_S_Radius`)))))))

(fn `AdjustImpactPoint`
  (returns (ImpactDirection :type "Vector Structure"))
  (if (`self.bIsAimAssistEnable`)
    ;[0 0.2091 1 0.25] Bullet Magnetism
    ;;[1 0 0.02461 0.25] Check if the feature is enable
    (if (`self.bEnableBulletMagnetism`)
      ;;[1 0 0.02461 0.25] Check if within the Bend Zone radius
      (if (< (`KismetMathLibrary.Distance2D` (`self.ClosestImpactPoint`) (`self.ScreenCenter`)) (`self.Adjusted_BM_Radius`))
        (if (or (not (`self.bTriggerLowVelocity`)) (<= (`self.LowVelocityTimer`) 0.5))
          ;[0 0.2748 1 0.33] Return Screen Center to Closest Impact Point from target in world
          (return (`.WorldDirection` (`GameplayStatics.DeprojectScreenToWorld` (`self.PlayerController`) (`self.ClosestImpactPoint`))))
          (else
            _)))))
  ;[0 0.2748 1 0.33] Return Screen Center to world impact
  (return (`.WorldDirection` (`GameplayStatics.DeprojectScreenToWorld` (`self.PlayerController`) (`self.ScreenCenter`)))))

(fn `AdjustPlayerAim`
  (params (ClosestEnemyLocation :type "Vector2D Structure"))
  (returns (AdjustedCrossHair :type "Vector2D Structure"))
  (bind _distancefromcenter (`self.DistanceFromCenter`))
  ;[1 1 1 0.33] Get distance from center of screen
  ;[1 0 0.02461 0.25] Check if in the Magnetic Zone
  (bind _output_get (set `self.DistanceFromCenter` (`KismetMathLibrary.Distance2D` ClosestEnemyLocation (`self.ScreenCenter`))))
  (if (< _output_get (`self.Adjusted_S_Radius`))
    (`|ExecutionSequence`
      (:`then_0`
        ;[0.946 1 0 0.25] Camera Snap
        ;;[1 0 0.02461 0.25] Check if target is Aligned with rotation
        (if (> (`KismetMathLibrary.DotProduct2D` (`self.InputDirectionNormalized`) (`KismetMathLibrary.Normal2D` (- (`local.ClosestEnemyLocation`) (`self.ScreenCenter`)))) (`self.Accuracy`))
          ;;[1 0 0.02461 0.25] Check if in the Snap Zone
          (if (< _distancefromcenter (`self.Adjusted_CS_Radius`))
            ;;[1 1 1 0.33] Slow Camera Speed and adjust rotation
            (if (`self.bEnableSnap`)
              (set `self.DecelerationRate` (* 0.2 (`self.CameraDecelerationMultiplier`)))
              (`self.AdjustPlayerRotation` (`local.ClosestEnemyLocation`) _distancefromcenter)
              (set `self.Assist State` "SNAP")
              (set `self.Color Current State` (struct :`R` 0.027451 :`G` 1.0 :`A` 1.0))
              (else
                ;;[1 1 1 0.33] Slow Down Camera Speed, depending on how close from the target is the crosshair
                (if (`self.bEnableStickiness`) :!label _label
                  (set `self.DecelerationRate` (`KismetMathLibrary.FClamp` (* (/ (`self.DistanceFromCenter`) (`self.Adjusted_S_Radius`)) (`self.CameraDecelerationMultiplier`)) 0.5))
                  (set `self.Assist State` "STICKNESS")
                  (set `self.Color Current State` (struct :`R` 1.0 :`B` 0.67451 :`A` 1.0)))))
            (else
              (goto _label)))
          (else
            ;;[1 1 1 0.33] Reset Camera Speed
            (set `self.DecelerationRate` 1.0))))
      (:`then_1`
        ;[0 0.2748 1 0.33] Return Closest Enemy Location
        (return (`local.ClosestEnemyLocation`))))
    (else
      ;[0 0.2748 1 0.33] Return Screen Center Location
      (return (`self.ScreenCenter`)))))

(fn `AdjustPlayerRotation`
  (params (TargetHit :type "Vector2D Structure") (Distance :type "Float (double-precision)"))
  (bind _playercontroller (`self.PlayerController`))
  (bind _returnvalue (* (/ Distance (`self.Adjusted_CS_Radius`)) (`self.CameraMagneticForce`)))
  (bind (_x _y) (`KismetMathLibrary.BreakVector2D` (* (`KismetMathLibrary.Normal2D` (- TargetHit (`self.ScreenCenter`))) (`KismetMathLibrary.MakeVector2D` _returnvalue _returnvalue))))
  ;[1 1 1 0.33] Apply Force to Yaw and Pitch inputs
  (`|ExecutionSequence`
    (:`then_0`
      (`PlayerController.AddYawInput` _playercontroller _x))
    (:`then_1`
      (`PlayerController.AddPitchInput` _playercontroller _y))))

(fn `Enemy Detection`
  (returns (`Hit?` :type Boolean) (HitScreenLocation :type "Vector2D Structure"))
  (locals (ClosestAlignedDirection :type "Float (double-precision)" :default 1.0) (ClosestDistance :type "Float (double-precision)" :default 999.0) (HitToScreen :type "Vector2D Structure") (ClosestHit :type "HitResult Structure"))
  (bind (_start _end) (`self.GetSphereTracePoints`))
  (bind (_bblockinghit _binitialoverlap _time _distance _location _impactpoint _normal _impactnormal _physmat _hitactor _hitcomponent) (`GameplayStatics.BreakHitResult` (`local.ClosestHit`)))
  ;[1 1 1 0.25] Get the Look Input and normalized it
  (set `self.InputDirectionNormalized` (`KismetMathLibrary.Normal2D` (`self.Input Direction`)))
  ;[1 1 1 0.25] Check if PAWN near crossHair
  (bind (_outhits _returnvalue) (`KismetSystemLibrary.SphereTraceMultiForObjects` _start _end (`self.SphereTraceRadius`) (`|MakeArray` "ObjectTypeQuery3" :!type "EObjectTypeQuery Enum")))
  ;;[1 0 0.02461 0.25] Check if hit
  (if _returnvalue
    (for _array_element _outhits
      (bind (_bblockinghit_2 _binitialoverlap_2 _time_2 _distance_2 _location_2 _impactpoint_2 _normal_2 _impactnormal_2 _physmat_2 _hitactor_2 _hitcomponent_2) (`GameplayStatics.BreakHitResult` _array_element))
      (bind _screenposition (`GameplayStatics.ProjectWorldToScreen` (`self.PlayerController`) (`KismetSystemLibrary.GetComponentBounds` _hitcomponent_2)))
      (bind _returnvalue_2 (- _screenposition (`self.ScreenCenter`)))
      (bind _returnvalue_3 (`KismetMathLibrary.VSize2D` _returnvalue_2))
      ;[1 0 0.02461 0.25] Check if it's the closest hit
      (if (< _returnvalue_3 (`local.ClosestDistance`))
        (set `local.ClosestDistance` _returnvalue_3)
        ;[1 0 0.02461 0.25] Check if in the BendZone
        (if (< _returnvalue_3 (`self.Adjusted_BM_Radius`))
          ;[1 1 1 0.33] Update closest Hit Position
          (set `local.HitToScreen` _screenposition :!label _label)
          (set `local.ClosestHit` _array_element)
          (set `self.ClosestImpactPoint` (`GameplayStatics.ProjectWorldToScreen` (`self.PlayerController`) _impactpoint_2))
          (else
            (bind _returnvalue_4 (- 1.0 (`KismetMathLibrary.DotProduct2D` (`self.InputDirectionNormalized`) (`KismetMathLibrary.Normal2D` _returnvalue_2))))
            ;[1 0 0.02461 0.25] Check which target is the most Aligned with the Aiming Direction
            (if (< _returnvalue_4 (`local.ClosestAlignedDirection`))
              (set `local.ClosestAlignedDirection` _returnvalue_4)
              (goto _label))))))
    ;[1 1 1 0.33] Adjust Circles only when new target
    (if (!= _hitcomponent (`self.CurrentTarget`))
      (set `self.CurrentTarget` _hitcomponent)
      (`self.AdjustCircles` (`KismetSystemLibrary.GetComponentBounds` _hitcomponent)))
    ;[1 1 1 0.33] Return Closest Hit To Screen Location
    (return true (`local.HitToScreen`))
    (else
      (return false (`self.ScreenCenter`)))))

(fn `GetPlayerController`
  ;[1 0 0.03774] Need to be replaced if MultiPlayer - Local Game
  (set `self.PlayerController` (`Pawn.GetLocalViewingPlayerController` (`Actor.Instigator` (`self.GetOwner`)))))

(fn `GetSphereTracePoints`
  (returns (Start :type "Vector Structure") (End :type "Vector Structure"))
  (bind (_worldposition _worlddirection) (`GameplayStatics.DeprojectScreenToWorld` (`self.PlayerController`) (`self.ScreenCenter`)))
  (return (+ _worldposition (* _worlddirection (`self.SphereTraceStartOffset`))) (+ _worldposition (* _worlddirection (`self.SphereTraceRange`)))))

(fn `Initialize HUD`
  (bind _playercontroller (`self.PlayerController`))
  (if (`self.bIsDebugActivated`)
    ;[1 1 1 0.25] Initialize HUD
    (`PlayerController.ClientSetHUD` _playercontroller "/Game/AdvancedAimAssist/Debug/AAA_HUD_Debug.AAA_HUD_Debug_C")
    (bind _output_get (set `self.AimAssistHUD` (cast `/Game/AdvancedAimAssist/Debug/AAA_HUD_Debug` (`PlayerController.GetHUD` _playercontroller) :!pure true)))
    (`/Game/AdvancedAimAssist/Debug/AAA_HUD_Debug.InitializeCircles` _output_get (`|MakeArray` (`self.BulletMagnetismRadius`) (`self.CameraSnapRadius`) (`self.SticknessRadius`)))
    (else
      ;[1 1 1 0.25] Reset HUD
      (`self.AimAssistHUD`
        (:`then`
          (set `self.AimAssistHUD` null)
          (`self.ResetHUD`))
        (:`else`)))))

(fn `ResetCamera`
  (set `self.AdjustCrossHairLocatin` (`self.ScreenCenter`))
  (set `self.DecelerationRate` 1.0)
  (set `self.Assist State` "")
  (set `self.Color Current State` (struct :`A` 1.0))
  (set `self.bIsAimAssistTriggered` false))

(fn `ResetHUD`
  (`PlayerController.ClientSetHUD` (`self.PlayerController`) "/Script/Engine.HUD"))

(fn `StartAimAssist`
  (set `self.bIsAimAssistEnable` true))

(fn `StopAimAssist`
  (set `self.bIsAimAssistEnable` false)
  (`self.ResetCamera`))

(fn `UpdateHUD`
  (bind _aimassisthud (`self.AimAssistHUD`))
  (if (`self.bIsDebugActivated`)
    (set `/Game/AdvancedAimAssist/Debug/AAA_HUD_Debug.CrossHairLocation` (`self.AdjustCrossHairLocatin`) _aimassisthud)
    (set `/Game/AdvancedAimAssist/Debug/AAA_HUD_Debug.ColorCurrentState` (`self.Color Current State`) _aimassisthud)
    (set `/Game/AdvancedAimAssist/Debug/AAA_HUD_Debug.AssistState` (`self.Assist State`) _aimassisthud)))

(fn `UpdateInputDirection`
  (params (InInputDirection :type "Vector2D Structure"))
  ;[1 0 0.02461 0.25] Check if Velocity is Near Zero
  (if (not (`KismetMathLibrary.IsNearlyZero2D` InInputDirection))
    ;[1 1 1 0.25] Update Rotation velocity
    (set `self.Input Direction` InInputDirection)
    (set `self.RotationVelocity` (`KismetMathLibrary.VSize2D` InInputDirection))
    ;[1 0 0.02461 0.25] Check if velocity too low
    (if (not (<= (`self.RotationVelocity`) 0.1))
      ;[1 1 1 0.25] Enable Aim Assist when Player is trying to aim properly
      (set `self.bIsAimAssistTriggered` true)
      ;;[1 0 0.05072 0.33] Reset Low Velocity Timer
      (set `self.bTriggerLowVelocity` false)
      (set `self.LowVelocityTimer` 0.0))
    (else
      ;[1 1 1 0.33] Trigger Low velocity to lock a target
      (set `self.bTriggerLowVelocity` true))))

(fn `UpdateLockState`
  (params (DeltaSec :type "Float (single-precision)"))
  ;[1 0 0.02461 0.25] Check how long since LockState is enable
  (set `self.LowVelocityTimer` (+ (`self.LowVelocityTimer`) DeltaSec))
  (if (not (<= (`self.LowVelocityTimer`) (`self.LockStateDuration`)))
    ;[1 1 1 0.25] Disable LockState and Reset Camera & HUD
    (`self.ResetCamera`)
    (set `self.bIsAimAssistTriggered` false)
    (set `self.bTriggerLowVelocity` false)
    (`self.UpdateHUD`)))

(fn `UpdateScreenCenter`
  (bind _returnvalue (`WidgetLayoutLibrary.GetViewportSize`))
  ;[1 1 1 0.33] Set the ScreenSize of the HUD
  (bind _aimassisthud (`self.AimAssistHUD`)
    (:`then`
      (set `/Game/AdvancedAimAssist/Debug/AAA_HUD_Debug.ScreenSize` _returnvalue _aimassisthud))
    (:`else`
      _))
  ;[1 1 1 0.33] Set Screen Center
  (set `self.ScreenCenter` (* _returnvalue (0.5 0.5))))