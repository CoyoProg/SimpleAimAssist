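; Shooting target actor with head, body and apple child actors that takes damage, falls over when killed and can respawn.
; Child hit components feed a shared life pool; at zero a death event fires, collision turns off and a timeline rotates the target down, reversed on respawn.
; Optional movement ping-pongs between origin and target position on Tick, pausing at each end.
; The construction script previews that path with a debug line.
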(event `self.ReceiveBeginPlay`
  ;[0.4885 0.005318 0 0.25] BEGIN PLAY
  ;;[1 1 1] Set Current Life
  (set `self.CurrentLife` (`self.MaxLife`))
  ;;[1 1 1] Get All Child Actors
  (for _array_element (`SceneComponent.GetChildrenComponents` (`self.DefaultSceneRoot`) false)
    (bind _aschild_actor_component (cast `ChildActorComponent` _array_element))
    ;;[1 1 1] Bind to On Hit Event
    (add `/Game/AdvancedAimAssist/Blueprints/Components/AAA_BP_HitComponent.OnHit` (`self.GetComponentByClass` (`ChildActorComponent.ChildActor` _aschild_actor_component) "/Game/AdvancedAimAssist/Blueprints/Components/AAA_BP_HitComponent.AAA_BP_HitComponent_C") (delegate `TakeDamage`))
    (set `self.OriginPosition` (`SceneComponent.K2_GetComponentLocation` (`self.DefaultSceneRoot`)))))

(event `TakeDamage`
  (params (DamageAmount :type Integer))
  ;[1 1 1] TAKE DAMAGE
  (bind _output_get (set `self.CurrentLife` (- (`self.CurrentLife`) DamageAmount)))
  ;[1 1 1] Check if Dead
  (if (<= _output_get 0)
    (`self.OnTargetDown` false)))

(event `OnTargetDown`
  (params (bBeingReset :type Boolean))
  (bind _defaultsceneroot (`self.DefaultSceneRoot`))
  (bind (_returnvalue_roll _returnvalue_pitch _returnvalue_yaw) (`KismetMathLibrary.BreakRotator` (`SceneComponent.K2_GetComponentRotation` _defaultsceneroot)))
  (set `self.bIsTargetDown` true)
  (if (not bBeingReset)
    (`self.OnDeathEvent`))
  (`self.SetActorEnableCollision` (`ChildActorComponent.ChildActor` (`self.Head`)) false)
  (`self.SetActorEnableCollision` (`ChildActorComponent.ChildActor` (`self.Body`)) false)
  (`self.SetActorEnableCollision` (`ChildActorComponent.ChildActor` (`self.Apple`)) false)
  ;[1 1 1] Rotate the Target
  (bind (_direction _rotationx) (`Timeline|Rotation` :!via `PlayFromStart` :!label _label)
    (:`Update`
      (`SceneComponent.K2_SetRelativeRotation` _defaultsceneroot (`KismetMathLibrary.MakeRotator` (* _rotationx -90.0) _returnvalue_pitch _returnvalue_yaw) false false))))

(event `RespawnTarget`
  (set `self.bIsTargetDown` false)
  (`self.Reset BodyParts`)
  (goto _label :!via `ReverseFromEnd`))

(event `self.ReceiveTick`
  (params (DeltaSeconds :type "Float (single-precision)"))
  ;[0.4885 0.005318 0 0.25] TICK
  ;;[0.5553 1 0 0.25] MOVING TARGET
  (if (`self.bIsMovingTarget`)
    ;;;[1 1 1] Move to target
    (`SceneComponent.K2_AddWorldOffset` (`self.DefaultSceneRoot`) (* (`KismetMathLibrary.GetDirectionUnitVector` (`SceneComponent.K2_GetComponentLocation` (`self.DefaultSceneRoot`)) (`self.NextPosition`)) (`self.Speed`)) false false)
    ;;;[1 1 1] Set Next Target Position
    (if (<= (`KismetMathLibrary.Vector_Distance` (`self.NextPosition`) (`SceneComponent.K2_GetComponentLocation` (`self.DefaultSceneRoot`))) (`self.Speed`))
      (`self.SetNextPosition`)
      ;;;[1 1 1] Delay when reaching target
      (set `self.bIsMovingTarget` false)
      (`KismetSystemLibrary.Delay` (`self.TimeBeforeNextPos`))
      (set `self.bIsMovingTarget` true))))

(fn `Reset BodyParts`
  (`self.SetActorEnableCollision` (`ChildActorComponent.ChildActor` (`self.Head`)) true)
  (`self.SetActorEnableCollision` (`ChildActorComponent.ChildActor` (`self.Body`)) true)
  (`self.SetActorEnableCollision` (`ChildActorComponent.ChildActor` (`self.Apple`)) true)
  (set `self.CurrentLife` (`self.MaxLife`)))

(fn `SetNextPosition`
  (locals (LastPosition :type "Vector Structure" :default (0.0 0.0 0.0)))
  (set `local.LastPosition` (`self.NextPosition`))
  (set `self.NextPosition` (`self.OriginPosition`))
  (set `self.OriginPosition` (`local.LastPosition`)))

(fn `UserConstructionScript`
  (if (`self.bIsMovingTarget`)
    ;[1 1 1] Draw Line
    (`KismetSystemLibrary.FlushPersistentDebugLines`)
    (bind _output_get (set `self.NextPosition` (`KismetMathLibrary.TransformLocation` (`self.GetTransform`) (`self.TargetPosition`))))
    (`KismetSystemLibrary.DrawDebugLine` (`SceneComponent.K2_GetComponentLocation` (`self.DefaultSceneRoot`)) _output_get (struct :`A` 1.0) 10.0 10.0)
    (else
      ;[1 1 1] Delet Lines
      (`KismetSystemLibrary.FlushPersistentDebugLines`))))