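; AAA_BP_BodyPart is a shooting target piece in the Advanced Aim Assist content that represents a bust body, head or apple.
; The construction script uses the BodyPart value to pick the matching static mesh for the Body component and applies the bust target material.
; On BeginPlay it copies BodyPart to its HitComponent, so that component knows which part it represents.
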(event `self.ReceiveBeginPlay`
  (set `/Game/AdvancedAimAssist/Blueprints/Components/AAA_BP_HitComponent.BodyPart` (`self.BodyPart`) (`self.HitComponent`)))

(fn `UserConstructionScript`
  (bind _body (`self.Body`))
  (switch `/Game/AdvancedAimAssist/Blueprints/ShootingTarget/AAA_E_BodyParts` (`self.BodyPart`)
    (:`NewEnumerator0`
      (`StaticMeshComponent.SetStaticMesh` _body "/Game/AdvancedAimAssist/ART/Meshes/SM_BustTarget_Bust.SM_BustTarget_Bust")
      (`PrimitiveComponent.SetMaterial` _body 0 "/Game/AdvancedAimAssist/ART/Meshes/M_BustTarget.M_BustTarget" :!label _label)
      (`PrimitiveComponent.SetMaterial` (`self.Body`) 0 "/Game/AdvancedAimAssist/ART/Meshes/M_BustTarget.M_BustTarget"))
    (:`NewEnumerator1`
      (`StaticMeshComponent.SetStaticMesh` _body "/Game/AdvancedAimAssist/ART/Meshes/SM_BustTarget_Head.SM_BustTarget_Head")
      (goto _label))
    (:`NewEnumerator2`
      (`StaticMeshComponent.SetStaticMesh` _body "/Game/AdvancedAimAssist/ART/Meshes/SM_Apple.SM_Apple")
      (`PrimitiveComponent.SetMaterial` (`self.Body`) 0 "/Game/AdvancedAimAssist/ART/Meshes/M_BustTarget.M_BustTarget"))))