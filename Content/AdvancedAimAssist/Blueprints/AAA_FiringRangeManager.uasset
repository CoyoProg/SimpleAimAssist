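; Firing range manager that runs a timed shooting trial, started when its hit component is struck.
; On BeginPlay it gathers shooting targets overlapping the range zone and listens for their deaths.
; Each wave raises a random selection from that pool, and a new wave follows once they are down or the wave lifetime expires.
; Text panels show countdown and score from the player's stats component, then accuracy when time runs out.
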(event `self.HitComponent.OnHit`
  (params (DamageAmount :type Integer))
  (if (not (`self.bIsGameStarted`))
    (`self.StartTrial`)
    (bind _playerstats (`self.PlayerStats`)
      (:`then`
        (add `/Game/AdvancedAimAssist/Blueprints/Components/AAA_BP_StatsComponent.OnScoreUpdated` _playerstats (delegate `UpdateCurentScore`)))
      (:`else`))))

(event `UpdateCurentScore`
  (`self.UpdateScore`))

(event `self.ReceiveBeginPlay`
  ;[1 0 0.02407 0.25] BEGIN PLAY
  (`KismetSystemLibrary.DelayUntilNextTick`)
  (for _array_element (`PrimitiveComponent.GetOverlappingActors` (`self.FiringRangeZone`) "/Game/AdvancedAimAssist/Blueprints/ShootingTarget/AAA_BP_ShootingTarget.AAA_BP_ShootingTarget_C")
    (bind _asaaa_bp_shooting_target (cast `/Game/AdvancedAimAssist/Blueprints/ShootingTarget/AAA_BP_ShootingTarget` _array_element))
    (`KismetArrayLibrary.Array_AddUnique` (`self.ShootingTargets`) _asaaa_bp_shooting_target)
    (add `/Game/AdvancedAimAssist/Blueprints/ShootingTarget/AAA_BP_ShootingTarget.OnDeathEvent` _asaaa_bp_shooting_target (delegate `OnTargetDown`))))

(event `OnTargetDown`
  (if (`self.bIsGameStarted`)
    (bind _result (`/Engine/EditorBlueprintResources/StandardMacros.DecrementInt` (`self.TargetsUpAmount`))
      (:`  `
        (if (< _result 0)
          (`self.NewWave`))))))

(event `self.ReceiveTick`
  (params (DeltaSeconds :type "Float (single-precision)"))
  ;[1 0 0.02407 0.25] TICK
  (if (`self.bIsGameStarted`)
    (`self.UpdateTimer` DeltaSeconds)))

(event `NewWave`
  (bind _currenttarget (`self.CurrentTarget`))
  ;[1 0 0.02407 0.25] NEW WAVE
  (set `self.CurrentWaveTimer` 0.0)
  (`KismetSystemLibrary.Delay` 0.25)
  (for _array_element _currenttarget
    (`KismetArrayLibrary.Array_AddUnique` (`self.ShootingTargets`) _array_element))
  (`KismetArrayLibrary.Array_Clear` _currenttarget)
  ;;[1 1 1] Amount of targets
  (bind _output_get (set `self.TargetsUpAmount` (`KismetMathLibrary.RandomInteger` 3)))
  (`self.SpawnNewTarget` _output_get))

(event `ResetWave`
  ;[1 0 0.02407 0.25] RESET WAVE
  (for _array_element (`self.CurrentTarget`)
    (`self.ResetTarget` _array_element))
  (`self.NewWave`))

(fn `ResetPannelTexts`
  (`TextRenderComponent.K2_SetText` (`self.ScoreValue`) (`|FormatText` "0000"))
  (`TextRenderComponent.K2_SetText` (`self.TimerValue`) (`|FormatText` "60,00"))
  (`TextRenderComponent.K2_SetText` (`self.Timer`) (`|FormatText` "TIMER")))

(fn `ResetTarget`
  (params (Target :type "/Game/AdvancedAimAssist/Blueprints/ShootingTarget/AAA_BP_ShootingTarget Object Reference"))
  (if (not (`/Game/AdvancedAimAssist/Blueprints/ShootingTarget/AAA_BP_ShootingTarget.bIsTargetDown` Target))
    (`/Game/AdvancedAimAssist/Blueprints/ShootingTarget/AAA_BP_ShootingTarget.OnTargetDown` Target true)))

(fn `ShowScore`
  (`TextRenderComponent.K2_SetText` (`self.Timer`) (`|FormatText` "ACCURACY"))
  (bind _playerstats (`self.PlayerStats`)
    (:`then`
      (`TextRenderComponent.K2_SetText` (`self.TimerValue`) (`KismetTextLibrary.Conv_DoubleToText` (`/Game/AdvancedAimAssist/Blueprints/Components/AAA_BP_StatsComponent.AccuracyStats` _playerstats) "HalfToEven")))
    (:`else`
      (`TextRenderComponent.K2_SetText` (`self.TimerValue`) (`|FormatText` "AAA_StatsComponent NOT FOUND")))))

(fn `SpawnNewTarget`
  (params (NewTargetAmount :type Integer))
  (locals (RandomIndex :type Integer :default 0))
  (bind _shootingtargets (`self.ShootingTargets`))
  (for _ (range (+ NewTargetAmount 1))
    (bind _output_get (set `local.RandomIndex` (`KismetMathLibrary.RandomInteger` (`KismetArrayLibrary.Array_Length` _shootingtargets))))
    (bind _output (`|GetArrayItem` _shootingtargets _output_get))
    (`KismetArrayLibrary.Array_AddUnique` (`self.CurrentTarget`) _output)
    (`KismetArrayLibrary.Array_RemoveItem` _shootingtargets _output))
  (for _array_element (`self.CurrentTarget`)
    (`/Game/AdvancedAimAssist/Blueprints/ShootingTarget/AAA_BP_ShootingTarget.RespawnTarget` _array_element)))

(fn `StartTrial`
  ;[1 1 1 0.25] Reset all targets that aren't down
  (for _array_element (`self.ShootingTargets`)
    (`self.ResetTarget` _array_element))
  (`|ExecutionSequence`
    (:`then_0`
      ;[1 1 1 0.25] Reset text panel
      (`self.ResetPannelTexts`)
      (set `self.CurrentScore` 0)
      (set `self.CurrentTimer` 60.0))
    (:`then_1`
      ;[1 1 1 0.25] Reset Stats Component
      (bind _output_get (set `self.PlayerStats` (`self.GetComponentByClass` (`GameplayStatics.GetPlayerPawn` 0) "/Game/AdvancedAimAssist/Blueprints/Components/AAA_BP_StatsComponent.AAA_BP_StatsComponent_C")))
      (`/Game/AdvancedAimAssist/Blueprints/Components/AAA_BP_StatsComponent.ResetStats` _output_get))
    (:`then_2`
      ;[1 1 1 0.25] Start the trial
      (set `self.bIsGameStarted` true)
      (`self.NewWave`))))

(fn `UpdateScore`
  (`TextRenderComponent.K2_SetText` (`self.ScoreValue`) (`KismetTextLibrary.Conv_IntToText` (`/Game/AdvancedAimAssist/Blueprints/Components/AAA_BP_StatsComponent.Score` (`self.PlayerStats`)) false false 4 10)))

(fn `UpdateTimer`
  (params (DeltaSec :type "Float (single-precision)"))
  (set `self.CurrentWaveTimer` (+ (`self.CurrentWaveTimer`) DeltaSec))
  (set `self.CurrentTimer` (- (`self.CurrentTimer`) DeltaSec))
  (if (<= (`self.CurrentTimer`) 0.0)
    (set `self.CurrentTimer` 60.0)
    (set `self.bIsGameStarted` false)
    (`self.ShowScore`)
    (else
      (`TextRenderComponent.K2_SetText` (`self.TimerValue`) (`KismetTextLibrary.Conv_DoubleToText` (`self.CurrentTimer`) "HalfToEven" false true 2 3 2 2))
      (if (>= (`self.CurrentWaveTimer`) (`self.WaveLifeTime`))
        (`self.ResetWave`)))))

(fn `UserConstructionScript`)